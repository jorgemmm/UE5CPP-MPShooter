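; BP_BlasterCharacter is the character Blueprint, which here holds only debug logic.
; Tick prints the Rolling state every frame, while BeginPlay and the construction script are empty.
; A disconnected FlipFlop would alternate the overhead WBP_OverHead widget between showing the player name and the net role, but it never runs.
; Unused nodes for movement speed, velocity and rolling readouts remain in the graph.
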(event EventBeginPlay)

(event EventTick
  (params (DeltaSeconds :type Float%20%28single-precision%29))
  (Development|PrintString (Utilities|String|ToString(Boolean) (Variables|Default|GetbRolling))))

(event Input|KeyboardEvents|N
  (params (Key :type Key%20Structure :default "None")))

(fn ConstructionScript)